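; BP_HighwaySpline is a level-building actor that lays highway meshes along an editable spline.
; Its construction script divides the spline by the middle mesh's X length, adding one spline mesh component per segment.
; The first segment uses the start mesh, the last the end mesh and others the middle mesh, with tangents clamped to segment length.
; Start and end mirroring logic is disconnected, and the event graph is empty.
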(fn `UserConstructionScript`
  (bind _spline (`self.Spline`))
  (bind _spline_2 (`self.Spline`))
  (bind (_returnvalue_min _returnvalue_max) (break `Box` (`StaticMesh.GetBoundingBox` (`self.MiddleMesh`))))
  (bind _returnvalue_x (`KismetMathLibrary.BreakVector` (+ (`KismetMathLibrary.Vector_GetAbs` _returnvalue_min) (`KismetMathLibrary.Vector_GetAbs` _returnvalue_max))))
  (bind _output_get (set `self.XLenght` _returnvalue_x))
  (bind _returnvalue (`KismetMathLibrary.FTrunc` (/ (`SplineComponent.GetSplineLength` (`self.Spline`)) _output_get)))
  (for _index (range (+ _returnvalue 1))
    (bind _returnvalue_2 (`AddComponent|NODE_AddSplineMeshComponent-0`))
    (bind _output_get_2 (set `self.ActiveMeshComponent` _returnvalue_2))
    (`SplineMeshComponent.SetForwardAxis` _output_get_2 "X" true)
    (if (== _index 0)
      (`StaticMeshComponent.SetStaticMesh` (`self.ActiveMeshComponent`) (`self.StartMesh`))
      (elif (== _index _returnvalue)
        (`StaticMeshComponent.SetStaticMesh` (`self.ActiveMeshComponent`) (`self.EndMesh`))
        (else
          (`StaticMeshComponent.SetStaticMesh` (`self.ActiveMeshComponent`) (`self.MiddleMesh`)))))
    (bind _returnvalue_3 (* _index (`self.XLenght`)))
    (bind _returnvalue_4 (* (+ _index 1) (`self.XLenght`)))
    (`SplineMeshComponent.SetStartAndEnd` (`self.ActiveMeshComponent`) (`SplineComponent.GetLocationAtDistanceAlongSpline` _spline_2 _returnvalue_3 "Local") (`KismetMathLibrary.ClampVectorSize` (`SplineComponent.GetTangentAtDistanceAlongSpline` _spline_2 _returnvalue_3 "Local") 0.0 (`self.XLenght`)) (`SplineComponent.GetLocationAtDistanceAlongSpline` _spline _returnvalue_4 "Local") (`KismetMathLibrary.ClampVectorSize` (`SplineComponent.GetTangentAtDistanceAlongSpline` _spline _returnvalue_4 "Local") 0.0 (`self.XLenght`)) false)))