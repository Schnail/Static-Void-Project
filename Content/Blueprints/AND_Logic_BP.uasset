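; AND gate logic actor that combines several boolean channel inputs, indexed by component ID, into one Pressed signal.
; InformChannel loops over NeededIDs, clearing Pressed on any false slot and storing the incoming value at the ComponentID index.
; Each slot is tested before its write, so the updated slot counts with its previous value.
; The result is relayed via InformChannelMessage to TargetClass actors tagged with ChannelName.
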(event `/Game/Interfaces/Channel_Interface.Inform Channel`
  (params (`Component ID` :type Integer) (`Float Value` :type "Float (double-precision)") (`Vec Value` :type "Vector Structure") (`Bool Value` :type Boolean))
  (bind _needed_ids (`self.Needed IDs`))
  (set `self.Pressed` true)
  (for (_array_element _array_index) (`self.Needed IDs`)
    (if (not _array_element)
      (set `self.Pressed` false))
    (if (== _array_index `Component ID`)
      (`KismetArrayLibrary.Array_Set` _needed_ids _array_index `Bool Value`)
      (else
        (`KismetArrayLibrary.Array_Set` _needed_ids _array_index _array_element))))
  (bind _outactors (`GameplayStatics.GetAllActorsOfClassWithTag` (`self.Target Class`) (`self.Channel Name`)))
  (message `/Game/Interfaces/Channel_Interface.Inform Channel` _outactors (`self.Component ID`) 0.0 (0.0 0.0 0.0) (`self.Pressed`)))

(fn `UserConstructionScript`)