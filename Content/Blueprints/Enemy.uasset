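; Enemy character that chases the player's Irie pawn, ragdolls when hit and respawns at its starting transform.
; Tick adds movement input toward Irie while horizontal distance lies within a set band, stopping up close or far away.
; A hit disables capsule collision and launches the physics-simulated mesh against the hit normal, scaled by hit strength.
; After a delay, it spawns a replacement and destroys itself, spawning an effect system where it was.
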(event `self.ReceiveBeginPlay`
  (set `self.Initial Transform` (`self.GetTransform`))
  (bind _asirie (cast `/Game/ThirdPerson/Blueprints/Irie` (`GameplayStatics.GetPlayerPawn` 0)))
  (set `self.Irie` _asirie))

(event `self.ReceiveTick`
  (params (DeltaSeconds :type "Float (single-precision)"))
  (bind _returnvalue (- (`self.K2_GetActorLocation` (`self.Irie`)) (`self.K2_GetActorLocation`)))
  (bind _returnvalue_2 (`KismetMathLibrary.VSizeXY` _returnvalue))
  (if (and (> _returnvalue_2 200.0) (< _returnvalue_2 5000.0))
    (`self.AddMovementInput` (`KismetMathLibrary.Normal` _returnvalue))))

(event `/Game/Interfaces/Hit_Interface.Component Hit`
  (params (`Hit Component` :type "ActorComponent Object Reference") (`Hit Normal` :type "Vector Structure") (`Hit Strength` :type "Float (double-precision)"))
  (bind _mesh (`self.Mesh`))
  (`PrimitiveComponent.SetCollisionProfileName` _mesh "Ragdoll" true)
  (`PrimitiveComponent.SetSimulatePhysics` _mesh true)
  (`PrimitiveComponent.AddVelocityChangeImpulseAtLocation` (`self.Mesh`) (* (`KismetMathLibrary.NegateVector` `Hit Normal`) (* `Hit Strength` 5.0)) (0.0 0.0 0.0) "None")
  (`PrimitiveComponent.SetCollisionProfileName` (`self.CapsuleComponent`) "NoCollision" true)
  (`KismetSystemLibrary.Delay` 3.0)
  (`|SpawnActorFromClass` "Enemy_C" (`self.Initial Transform`) "Undefined" "MultiplyWithRoot" null null)
  (add `self.OnDestroyed` (delegate `OnDestroyed_Event`))
  (`self.K2_DestroyActor`))

(event `OnDestroyed_Event` :!signature `self.OnDestroyed`
  (params (DestroyedActor :type "Actor Object Reference"))
  (`NiagaraFunctionLibrary.SpawnSystemAtLocation` null (`self.K2_GetActorLocation`) :!label _label))

(event `self.ReceiveDestroyed`
  (goto _label))

(fn `UserConstructionScript`)