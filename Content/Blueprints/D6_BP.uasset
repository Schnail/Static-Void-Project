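; D6_BP is a physics-driven six-sided die that plays an explode effect on its top face when it stops.
; A hit pushes the mesh against the hit normal with slight lift, scaled by strength, then sets IsRolling a tick later.
; Tick waits for zero velocity, then uses a dot product with world up to pick among six face arrows.
; RollDice applies a given impulse but never sets IsRolling.
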(event `self.ReceiveBeginPlay`
  (set `self.Sides` (`|MakeArray` (`self.Arrow1`) (`self.Arrow2`) (`self.Arrow3`) (`self.Arrow4`) (`self.Arrow5`) (`self.Arrow6`))))

(event `self.ReceiveTick`
  (params (DeltaSeconds :type "Float (single-precision)"))
  (if (`self.IsRolling`)
    (if (`KismetMathLibrary.EqualExactly_VectorVector` (`SceneComponent.GetComponentVelocity` (`self.StaticMesh`)))
      (set `self.IsRolling` false)
      (for _array_element (`self.Sides`)
        (if (> (`KismetMathLibrary.Dot_VectorVector` (`SceneComponent.GetForwardVector` _array_element) (0.0 0.0 1.0)) 0.5)
          (`NiagaraFunctionLibrary.SpawnSystemAttached` "/Game/VFX/Explode.Explode" _array_element "None" (0.0 0.0 0.0) (struct) "KeepRelativeOffset"))))))

(event `/Game/Interfaces/Hit_Interface.Component Hit`
  (params (`Hit Component` :type "ActorComponent Object Reference") (`Hit Normal` :type "Vector Structure") (`Hit Strength` :type "Float (double-precision)"))
  (`PrimitiveComponent.AddVelocityChangeImpulseAtLocation` (`self.StaticMesh`) (* (+ (`KismetMathLibrary.NegateVector` `Hit Normal`) (0.0 0.0 0.2)) `Hit Strength`) (0.0 0.0 0.0) "None")
  (`KismetSystemLibrary.DelayUntilNextTick`)
  (set `self.IsRolling` true))

(fn `Roll Dice`
  (params (`Roll Vector` :type "Vector Structure"))
  (`PrimitiveComponent.AddVelocityChangeImpulseAtLocation` (`self.StaticMesh`) `Roll Vector` (0.0 0.0 0.0) "None"))

(fn `UserConstructionScript`)