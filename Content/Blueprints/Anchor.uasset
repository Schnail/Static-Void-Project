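; Anchor actor that pulls the player's Irie character to itself when its component registers a hit.
; Two pyramid components spin continuously through a fixed local rotation each Tick, independent of delta time.
; Any hit, regardless of the hitting actor, stores Irie's location and restarts the Grab timeline, which lerps Irie without sweep to a point below the anchor.
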(event `self.ReceiveBeginPlay`)

(event `self.ReceiveTick`
  (params (DeltaSeconds :type "Float (single-precision)"))
  (`SceneComponent.K2_AddLocalRotation` (`self.Lower Pyr`) (struct :`Yaw` 2.0) false false)
  (`SceneComponent.K2_AddLocalRotation` (`self.Upper Pyr`) (struct :`Yaw` 2.0) false false))

(event `/Game/Interfaces/Hit_Interface.Component Hit`
  (params (`Hit Component` :type "ActorComponent Object Reference") (`Hit Normal` :type "Vector Structure") (`Hit Strength` :type "Float (double-precision)"))
  (bind _asirie (cast `/Game/ThirdPerson/Blueprints/Irie` (`GameplayStatics.GetPlayerCharacter` 0)))
  (bind _output_get (set `self.NewVar` (`self.K2_GetActorLocation` _asirie)))
  (bind (_direction _grabdistance) (`Timeline|grab` :!via `PlayFromStart`)
    (:`Update`
      (`self.K2_SetActorLocation` _asirie (`KismetMathLibrary.VLerp` _output_get (- (`self.K2_GetActorLocation`) (0.0 0.0 200.0)) _grabdistance) false false))))

(fn `UserConstructionScript`)