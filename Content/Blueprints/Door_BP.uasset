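; Door actor that opens its Gate only while every input on its channel reports true.
; It tags itself with ChannelName on BeginPlay and receives InformChannel events, storing each component's state in the NeededIDs boolean array at the index matching its ID.
; Any false entry reverses the Open timeline and all true plays it, sliding the Gate between the ClosedPos and OpenPos relative locations.
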(event `self.ReceiveBeginPlay`
  (set `self.Tags` (`|MakeArray` (`self.Channel Name`))))

(event `/Game/Interfaces/Channel_Interface.Inform Channel`
  (params (`Channel Name` :type Name) (`Component ID` :type Integer) (`Float Value` :type "Float (double-precision)") (`Vec Value` :type "Vector Structure") (`Bool Value` :type Boolean))
  (for (_ _array_index) (`self.Needed IDs`)
    (if (== `Component ID` _array_index)
      (`KismetArrayLibrary.Array_Set` (`self.Needed IDs`) _array_index `Bool Value`)))
  (if (`KismetArrayLibrary.Array_Contains` (`self.Needed IDs`))
    (bind (_direction _openness) (`Timeline|Open` :!via `Reverse` :!label _label)
      (:`Update`
        (`SceneComponent.K2_SetRelativeLocation` (`self.Gate`) (`KismetMathLibrary.VLerp` (`SceneComponent.RelativeLocation` (`self.ClosedPos`)) (`SceneComponent.RelativeLocation` (`self.OpenPos`)) _openness) false false)))
    (else
      (goto _label))))

(fn `UserConstructionScript`)