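; Pressure plate that detects objects in its Box and signals actors on a named channel.
; Begin overlap presses it unless already pressed at WeightThreshold, so it can press below threshold; end overlap releases it when the component count minus one drops below threshold.
; State changes swap four light materials, move the Plate and send InformChannelMessage with ComponentID and Pressed to TargetClass actors tagged ChannelName.
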(event `self.Box.OnComponentEndOverlap`
  (params (OverlappedComponent :type "PrimitiveComponent Object Reference") (OtherActor :type "Actor Object Reference") (OtherComp :type "PrimitiveComponent Object Reference") (OtherBodyIndex :type Integer))
  (bind _channel_name (`self.Channel Name`))
  (if (and (< (- (`KismetArrayLibrary.Array_Length` (`PrimitiveComponent.GetOverlappingComponents` (`self.Box`))) 1) (`self.weight threshold`)) (`self.Pressed`))
    (set `self.Pressed` false)
    (`PrimitiveComponent.SetMaterial` (`self.Light4`) 0 "/Game/Materials/Cell_HitObject.Cell_HitObject")
    (`PrimitiveComponent.SetMaterial` (`self.Light3`) 0 "/Game/Materials/Cell_HitObject.Cell_HitObject")
    (`PrimitiveComponent.SetMaterial` (`self.Light2`) 0 "/Game/Materials/Cell_HitObject.Cell_HitObject")
    (`PrimitiveComponent.SetMaterial` (`self.Light1`) 0 "/Game/Materials/Cell_HitObject.Cell_HitObject")
    (`SceneComponent.K2_SetRelativeLocation` (`self.Plate`) (0.0 0.0 0.0) false false)
    (bind _outactors (`GameplayStatics.GetAllActorsOfClassWithTag` (`self.Target Class`) _channel_name :!label _label))
    (message `/Game/Interfaces/Channel_Interface.Inform Channel` _outactors _channel_name (`self.Component ID`) 0.0 (0.0 0.0 0.0) (`self.Pressed`))))

(event `self.Box.OnComponentBeginOverlap`
  (params (OverlappedComponent :type "PrimitiveComponent Object Reference") (OtherActor :type "Actor Object Reference") (OtherComp :type "PrimitiveComponent Object Reference") (OtherBodyIndex :type Integer) (bFromSweep :type Boolean) (SweepResult :type "HitResult Structure (by ref)"))
  (if (not (and (>= (- (`KismetArrayLibrary.Array_Length` (`PrimitiveComponent.GetOverlappingComponents` (`self.Box`))) 1) (`self.weight threshold`)) (`self.Pressed`)))
    (set `self.Pressed` true)
    (`PrimitiveComponent.SetMaterial` (`self.Light4`) 0 "/Game/Materials/Cell_HitObject_Active.Cell_HitObject_Active")
    (`PrimitiveComponent.SetMaterial` (`self.Light3`) 0 "/Game/Materials/Cell_HitObject_Active.Cell_HitObject_Active")
    (`PrimitiveComponent.SetMaterial` (`self.Light2`) 0 "/Game/Materials/Cell_HitObject_Active.Cell_HitObject_Active")
    (`PrimitiveComponent.SetMaterial` (`self.Light1`) 0 "/Game/Materials/Cell_HitObject_Active.Cell_HitObject_Active")
    (`SceneComponent.K2_SetRelativeLocation` (`self.Plate`) (0.0 0.0 -4.0) false false)
    (goto _label)))

(fn `UserConstructionScript`)