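; Actor for a 2x2 Rubik's cube puzzle that turns a side when one of its Face-tagged components is hit.
; Marker components whose axes match the face's up vector select their parent cubes to rotate.
; A timeline lerps those cubes 90 degrees around that axis from cached start rotations.
; At start and after each turn, the solved check compares one piece's forward vector to the average of all eight, updating the display text.
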(event `self.ReceiveBeginPlay`
  (set `self.Vecs` (`|MakeArray` (`self.BRO_Vec`) (`self.BYR_Vec`) (`self.YGV_Vec`) (`self.BGO_Vec`) (`self.GOV_Vec`) (`self.BYG_Vec`) (`self.ROV_Vec`) (`self.RYV_Vec`)))
  (bind _solved (`self.isSolved` :!label _label))
  (`self.Update text` _solved))

(event `After Turn`
  (goto _label))

(event `/Game/Interfaces/Hit_Interface.Component Hit`
  (params (`Hit Component` :type "PrimitiveComponent Object Reference") (`Hit Normal` :type "Vector Structure") (`Hit Strength` :type "Float (double-precision)"))
  (bind _returnvalue (`SceneComponent.GetUpVector` `Hit Component`))
  (if (`ActorComponent.ComponentHasTag` `Hit Component` "Face")
    (bind _cubes (`self.Get relevant Cubes` _returnvalue))
    (for (_array_element _array_index) _cubes
      (`KismetArrayLibrary.Array_Set` (`self.CubesRotations`) _array_index (`SceneComponent.K2_GetComponentRotation` _array_element) true))
    (bind (_direction _espargus) (`Timeline|Smooth Rotate` :!via `PlayFromStart`)
      (:`Update`
        (for (_array_element_2 _array_index_2) _cubes
          (bind _output (`|GetArrayItem` (`self.CubesRotations`) _array_index_2))
          (`SceneComponent.K2_SetWorldRotation` _array_element_2 (`KismetMathLibrary.RLerp` _output (`KismetMathLibrary.ComposeRotators` _output (`KismetMathLibrary.RotatorFromAxisAndAngle` _returnvalue 90.0)) _espargus true) false false)))
      (:`Finished`
        (`self.After Turn`)))))

(fn `Get relevant Cubes`
  (params (RotationAxis :type "Vector Structure"))
  (returns (Cubes :type "Array of SceneComponent Object Reference"))
  (locals (`Alligned Cubes` :type "Array of SceneComponent Object Reference"))
  (set `local.Alligned Cubes` (`|MakeArray` null null null null :!type "SceneComponent Object Reference"))
  (for _array_element (`self.Vecs`)
    (if (or (== (`SceneComponent.GetForwardVector` _array_element) RotationAxis :`ErrorTolerance` 0.01) (== (`SceneComponent.GetUpVector` _array_element) RotationAxis :`ErrorTolerance` 0.01) (== RotationAxis (`SceneComponent.GetRightVector` _array_element) :`ErrorTolerance` 0.01))
      (`KismetArrayLibrary.Array_Add` (`local.Alligned Cubes`) (`SceneComponent.GetAttachParent` _array_element))))
  (return (`local.Alligned Cubes`)))

(fn `isSolved`
  (returns (Solved :type Boolean))
  (bind _returnvalue (`SceneComponent.GetForwardVector` (`self.Rubix2x2_YGV`)))
  (return (== _returnvalue (/ (+ _returnvalue (`SceneComponent.GetForwardVector` (`self.Rubix2x2_RYV`)) (`SceneComponent.GetForwardVector` (`self.Rubix2x2_ROV`)) (`SceneComponent.GetForwardVector` (`self.Rubix2x2_GOV`)) (`SceneComponent.GetForwardVector` (`self.Rubix2x2_BYG`)) (`SceneComponent.GetForwardVector` (`self.Rubix2x2_BRY`)) (`SceneComponent.GetForwardVector` (`self.Rubix2x2_BRO`)) (`SceneComponent.GetForwardVector` (`self.Rubix2x2_BGO`))) 8.0) :`ErrorTolerance` 0.01)))

(fn `Update text`
  (params (Solved :type Boolean))
  (if Solved
    (set `self.DisplayText` "Cube is solved")
    (else
      (set `self.DisplayText` "Cube is unsolved")))
  (`TextRenderComponent.K2_SetText` (`self.Display`) (`self.DisplayText`)))

(fn `UserConstructionScript`)