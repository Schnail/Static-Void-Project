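; Button actor that works as a toggle switch, changing state each time its component is hit.
; Each hit flips the Pressed flag and swaps the Cube's material between active and inactive variants.
; It then reports the new state to its Target through InformChannelMessage, tagged with a channel name and component ID.
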(event `/Game/Interfaces/Hit_Interface.Component Hit`
  (params (`Hit Component` :type "ActorComponent Object Reference") (`Hit Normal` :type "Vector Structure") (`Hit Strength` :type "Float (double-precision)"))
  (bind _cube (`self.Cube`))
  (if (`self.Pressed`)
    (set `self.Pressed` false)
    (`PrimitiveComponent.SetMaterial` _cube 0 "/Game/Materials/Cell_HitObject.Cell_HitObject")
    (else
      (set `self.Pressed` true)
      (`PrimitiveComponent.SetMaterial` _cube 0 "/Game/Materials/Cell_HitObject_Active.Cell_HitObject_Active")))
  (message `/Game/Interfaces/Channel_Interface.Inform Channel` (`self.Target`) (`self.Channel Name`) (`self.Component ID`) 0.0 (0.0 0.0 0.0) (`self.Pressed`)))

(fn `UserConstructionScript`)