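; Bridge actor that extends or retracts along its Y axis when its Bridge component registers a hit.
; The hit checks the current Y scale, reversing the ExpandBridge timeline past the threshold and playing it otherwise.
; Timeline updates lerp relative scale and location together, so the bridge grows from a fixed near edge rather than from its center.
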(event `/Game/Interfaces/Hit_Interface.Component Hit`
  (params (`Hit Component` :type "ActorComponent Object Reference") (`Hit Normal` :type "Vector Structure") (`Hit Strength` :type "Float (double-precision)"))
  (bind _bridge (`self.Bridge`))
  (if (== `Hit Component` _bridge)
    (if (> (.y (`SceneComponent.RelativeScale3D` _bridge)) 10.0)
      (bind (_direction _newtrack_0) (`Timeline|Expand Bridge` :!via `Reverse` :!label _label)
        (:`Update`
          (`SceneComponent.SetRelativeScale3D` _bridge (`KismetMathLibrary.VLerp` (3.0 1.0 0.5) (3.0 20.0 0.5) _newtrack_0))
          (`SceneComponent.K2_SetRelativeLocation` _bridge (`KismetMathLibrary.VLerp` (0.0 50.0 -25.0) (0.0 1000.0 -25.0) _newtrack_0) false false)))
      (else
        (goto _label)))))

(fn `UserConstructionScript`)