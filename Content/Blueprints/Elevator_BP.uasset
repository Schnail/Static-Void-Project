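; Elevator actor that moves a platform between Start and End points in response to a boolean channel signal.
; BeginPlay sets the actor's tags to its ChannelName.
; InformChannel plays a timeline on true and reverses it on false.
; The timeline track drives a lerp between the two points' world locations, setting the platform's position without sweep.
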(event `self.ReceiveBeginPlay`
  (set `self.Tags` (`|MakeArray` (`self.Channel Name`))))

(event `/Game/Interfaces/Channel_Interface.Inform Channel`
  (params (`Channel Name` :type Name) (`Component ID` :type Integer) (`Float Value` :type "Float (double-precision)") (`Vec Value` :type "Vector Structure") (`Bool Value` :type Boolean))
  (if `Bool Value`
    (bind (_direction _newtrack_0) (`Timeline|Timeline` :!label _label)
      (:`Update`
        (`SceneComponent.K2_SetWorldLocation` (`self.Platform`) (`KismetMathLibrary.VLerp` (`SceneComponent.K2_GetComponentLocation` (`self.Start`)) (`SceneComponent.K2_GetComponentLocation` (`self.End`)) _newtrack_0) false false)))
    (else
      (goto _label :!via `Reverse`))))

(fn `UserConstructionScript`)