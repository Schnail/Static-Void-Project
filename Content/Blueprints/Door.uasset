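; Door Blueprint that toggles a gate open or closed when its InformChannel event fires.
; The event prints a debug "Hello", checks the channel name, then flips GateOpen and plays or reverses the Open timeline.
; The timeline's Openness track lerps the Gate's relative location between the OpenPos and ClosedPos component locations, with sweep enabled.
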(event `/Game/Interfaces/Channel_Interface.Inform Channel`
  (params (`Channel Name` :type Name) (`Component ID` :type Integer) (`Float Value` :type "Float (double-precision)") (`Vec Value` :type "Vector Structure") (`Bool Value` :type Boolean))
  (`KismetSystemLibrary.PrintString` "Hello")
  (if (== `Channel Name` (`self.Channel Name`))
    (if (`self.Gate Open`)
      (set `self.Gate Open` false)
      (bind (_direction _openness) (`Timeline|Open` :!via `Reverse` :!label _label)
        (:`Update`
          (`SceneComponent.K2_SetRelativeLocation` (`self.Gate`) (`KismetMathLibrary.VLerp` (`SceneComponent.RelativeLocation` (`self.OpenPos`)) (`SceneComponent.RelativeLocation` (`self.ClosedPos`)) _openness) true false)))
      (else
        (set `self.Gate Open` true)
        (goto _label)))))

(fn `UserConstructionScript`)